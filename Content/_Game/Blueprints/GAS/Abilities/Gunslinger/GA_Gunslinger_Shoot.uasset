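; Gunslinger gameplay ability that fires a burst of rifle shots of random length, from one up to MaxCounter + 1 montage loops.
; Each loop plays the rifle fire montage and waits for the Event.Montage.FireBolt gameplay event to spawn a projectile without pitch modification.
; Completed, blend-out, interrupted and cancelled callbacks all advance the counter, replaying the montage or ending the ability once the rolled count is exceeded.
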(event `self.K2_ActivateAbility`
  (set `self.CurrentCounter` 1)
  (set `self.Counter` (`KismetMathLibrary.RandomIntegerInRange` 1 (+ (`self.MaxCounter`) 1)))
  (`AbilityTask_PlayMontageAndWait.CreatePlayMontageAndWaitProxy` "None" "/Game/_Game/Blueprints/Character/Animations/Montages/ShootRifle/MM_Rifle_Fire_Montage.MM_Rifle_Fire_Montage" :!label _label
    (:`then`
      (`AbilityTask_WaitGameplayEvent.WaitGameplayEvent` (struct :`TagName` "Event.Montage.FireBolt") null
        (:`EventReceived`
          (`self.SpawnProjectile` 0.0 false))))
    (:`OnCompleted`
      (`/Engine/EditorBlueprintResources/StandardMacros.IncrementInt` (`self.CurrentCounter`) :!label _label_2
        (:`  `
          (if (<= (`self.CurrentCounter`) (`self.Counter`))
            (goto _label)
            (else
              (`self.K2_EndAbility`))))))
    (:`OnBlendOut`
      (goto _label_2))
    (:`OnInterrupted`
      (goto _label_2))
    (:`OnCancelled`
      (goto _label_2))))