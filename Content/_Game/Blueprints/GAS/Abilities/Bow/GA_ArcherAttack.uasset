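; Gameplay ability for an archer's bow attack, playing the shot montage and firing a projectile.
; Once the montage starts, it waits in parallel for gameplay events that time each stage of the shot.
; The arrow creation, draw and fake-arrow removal events send messages to the avatar, while the FireBolt event spawns the projectile without pitch adjustment.
; The ability ends when the montage completes, is interrupted or is cancelled.
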(event `self.K2_ActivateAbility`
  (bind _returnvalue (`self.GetAvatarActorFromActorInfo`))
  (`AbilityTask_PlayMontageAndWait.CreatePlayMontageAndWaitProxy` "None" "/Game/_Game/Blueprints/Character/Animations/Montages/Bow/M_Bow_ShotArrow.M_Bow_ShotArrow"
    (:`then`
      (`|ExecutionSequence`
        (:`then_0`
          (`AbilityTask_WaitGameplayEvent.WaitGameplayEvent` (struct :`TagName` "Archer.MakeArrow") null
            (:`EventReceived`
              (message `/Game/_Game/Blueprints/Interfaces/BPI_AI_Interface.Archer_MakeArrow` _returnvalue))))
        (:`then_1`
          (`AbilityTask_WaitGameplayEvent.WaitGameplayEvent` (struct :`TagName` "Archer.Draw") null
            (:`EventReceived`
              (message `/Game/_Game/Blueprints/Interfaces/BPI_AI_Interface.Archer_Draw` _returnvalue))))
        (:`then_2`
          (`AbilityTask_WaitGameplayEvent.WaitGameplayEvent` (struct :`TagName` "Archer.DeleteFakeArrow") null
            (:`EventReceived`
              (message `/Game/_Game/Blueprints/Interfaces/BPI_AI_Interface.Archer_DeleteFakeArrow` _returnvalue))))
        (:`then_3`
          (`AbilityTask_WaitGameplayEvent.WaitGameplayEvent` (struct :`TagName` "Event.Montage.FireBolt") null
            (:`EventReceived`
              (`self.SpawnProjectile` 0.0 false)
              (`KismetSystemLibrary.PrintString` "SPAWN PROJECTILE"))))))
    (:`OnCompleted`
      (`self.K2_EndAbility` :!label _label))
    (:`OnInterrupted`
      (goto _label))
    (:`OnCancelled`
      (goto _label))))