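; Gameplay ability that summons random minions around the caster with a magic staff montage.
; On the montage's gameplay event (tagged FireBolt), it shuffles spawn locations and marks each with a Niagara aura.
; A delayed loop spawns minions one by one, facing away from the caster with a spawn montage, clearing auras after the first delay.
; Minion count is messaged to the avatar on spawn and destruction; the ability ends when locations run out.
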(event `self.K2_ActivateAbility`
  (bind _returnvalue (+ (`|GetArrayItem` (`self.SpawnLocations`) (`self.SpanLocationIndex`)) (0.0 0.0 90.0)))
  (set `self.SpanLocationIndex` 0)
  (`AbilityTask_PlayMontageAndWait.CreatePlayMontageAndWaitProxy` "None" "/Game/_Game/Blueprints/Character/Animations/Montages/MagicStaff/M_MagicStaffSummon.M_MagicStaffSummon" 1.0 "None" false
    (:`then`
      (`AbilityTask_WaitGameplayEvent.WaitGameplayEvent` (struct :`TagName` "Event.Montage.FireBolt") null
        (:`EventReceived`
          (bind _returnvalue_2 (`self.GetSpawnLocations`))
          (bind _output_get (set `self.SpawnLocations` _returnvalue_2))
          (`KismetArrayLibrary.Array_Shuffle` _output_get)
          (for _array_element _output_get
            (bind _returnvalue_3 (`NiagaraFunctionLibrary.SpawnSystemAtLocation` "/Game/AdvancedMagicFX12/particles/Niagara/NS_ky_aura.NS_ky_aura" _array_element (struct) (0.5 0.5 0.5)))
            (`KismetArrayLibrary.Array_AddUnique` (`self.NiagaraArray`) _returnvalue_3))
          (if (< (`self.SpanLocationIndex`) (`KismetArrayLibrary.Array_Length` (`self.SpawnLocations`))) :!label _label
            (bind _returnvalue_4 (`|SpawnActorFromClass` (`self.GetRandomMinionClass`) (`KismetMathLibrary.MakeTransform` _returnvalue (`KismetMathLibrary.FindLookAtRotation` (`Actor.K2_GetActorLocation` (`self.GetAvatarActorFromActorInfo`)) _returnvalue)) "AlwaysSpawn" "MultiplyWithRoot" null null))
            (add `Actor.OnDestroyed` _returnvalue_4 (delegate `OnDestroyed_Event`))
            (message `CombatInterface.SetMinionCount` (`self.GetAvatarActorFromActorInfo`) 1)
            (bind _ascharacter (cast `Character` _returnvalue_4))
            (`/Engine/EditorBlueprintResources/StandardMacros.IsValid` _ascharacter
              (:`Is Valid`
                (`|PlayMontage` (`Character.Mesh` _ascharacter) "/Game/_Game/Blueprints/Character/Animations/Montages/SSH/M_SSH_Spawn.M_SSH_Spawn"
                  (:`then`
                    (`/Engine/EditorBlueprintResources/StandardMacros.IncrementInt` (`self.SpanLocationIndex`)
                      (:`  `
                        (`KismetSystemLibrary.Delay` 0.2)
                        (for _array_element_2 (`self.NiagaraArray`)
                          (`ActorComponent.Deactivate` _array_element_2))
                        (`KismetArrayLibrary.Array_Clear` (`self.NiagaraArray`))
                        (goto _label)))))))
            (else
              (`self.K2_EndAbility`))))))))

(event `OnDestroyed_Event`
  (params (DestroyedActor :type "Actor Object Reference"))
  (message `CombatInterface.SetMinionCount` (`self.GetAvatarActorFromActorInfo`) -1))