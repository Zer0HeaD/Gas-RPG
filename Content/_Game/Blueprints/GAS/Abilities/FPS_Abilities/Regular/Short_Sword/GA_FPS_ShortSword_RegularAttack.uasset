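; Gameplay ability for the first-person short sword's regular attack, which runs a combo graph and ends when that graph finishes.
; While the combo runs, it listens for Event.Hit gameplay events and loops over the actors in the target data.
; Each hit actor supplies its own Niagara effect and sound through interface calls, which play at that target's hit location, with errors reported for invalid assets.
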(event `self.K2_ActivateAbility`
  (`ComboGraphAbilityTask_StartGraph.CreateStartComboGraph` "/Game/_Game/Blueprints/GAS/Abilities/FPS_Abilities/Regular/Short_Sword/CG_FPS_ShortSword_RegularAttack.CG_FPS_ShortSword_RegularAttack"
    (:`then`
      ; Assign on hit event, go through array of enemies. On hit we play vfx and sound for each enemy
      (bind (_asynctaskproxy _payload) (`AbilityTask_WaitGameplayEvent.WaitGameplayEvent` (struct :`TagName` "Event.Hit") null)
        (:`EventReceived`
          (bind (_eventtag _instigator _target _optionalobject _optionalobject2 _contexthandle _instigatortags _targettags _eventmagnitude _targetdata) (break `GameplayEventData` _payload))
          (for (_array_element _array_index) (`AbilitySystemBlueprintLibrary.GetAllActorsFromTargetData` _targetdata)
            (`/Engine/EditorBlueprintResources/StandardMacros.IsValid` _array_element
              (:`Is Valid`
                (bind _returnvalue (message `CombatInterface.GetHitEffect` _array_element))
                (`/Engine/EditorBlueprintResources/StandardMacros.IsValid` _returnvalue
                  (:`Is Valid`
                    (bind (_bblockinghit _binitialoverlap _time _distance _location _impactpoint) (`GameplayStatics.BreakHitResult` (`AbilitySystemBlueprintLibrary.GetHitResultFromTargetData` _targetdata _array_index)))
                    (`NiagaraFunctionLibrary.SpawnSystemAtLocation` _returnvalue _impactpoint)
                    (bind _returnvalue_2 (message `CombatInterface.GetHitSound` _array_element))
                    (`/Engine/EditorBlueprintResources/StandardMacros.IsValid` _returnvalue_2
                      (:`Is Valid`
                        (`GameplayStatics.PlaySoundAtLocation` _returnvalue_2 _location (struct) 1.0 1.0 0.0 null null null null))
                      (:`Is Not Valid`
                        (`/Game/_Game/Blueprints/Libraries/BP_MicroLibrary.ErrorMessage` "INVALID SOUND SYSTEM VIA INTERFACE!"))))
                  (:`Is Not Valid`
                    (`/Game/_Game/Blueprints/Libraries/BP_MicroLibrary.ErrorMessage` "INVALID NIAGARA SYSTEM VIA INTERFACE!")))))))))
    (:`OnGraphEnd`
      (`self.K2_EndAbility`))))

(event `self.K2_OnEndAbility`
  (params (bWasCancelled :type Boolean)))