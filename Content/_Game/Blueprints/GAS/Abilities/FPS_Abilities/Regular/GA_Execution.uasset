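; GA_Execution is a gameplay ability that performs a fist execution on a victim.
; It passes the Fist_Execution row from DT_Execution to the avatar's execution component, which starts the execution and supplies the victim.
; With a valid victim, it waits for the Event.Montage.FireBolt gameplay event, applies the CalculateDamage effect spec to the victim's ability system, then ends.
; A missing component or victim ends the ability immediately.
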(event `self.K2_ActivateAbility`
  (bind _inmes (message `/Game/_Game/Blueprints/Interfaces/BPI_PlayerCharacterUtility.GetExecutionComponent` (`self.GetAvatarActorFromActorInfo`)))
  (`/Engine/EditorBlueprintResources/StandardMacros.IsValid` _inmes
    (:`Is Valid`
      (bind _returnvalue (`|GetDataTableRow` "/Game/MES/DataTable/DT_Execution.DT_Execution" "Fist_Execution")
        (:`then`
          (`/Game/MES/Blueprint/Component/MES.Start Execution` _inmes _returnvalue 0)
          (bind _victim (`/Game/MES/Blueprint/Component/MES.Victim` _inmes))
          (`/Engine/EditorBlueprintResources/StandardMacros.IsValid` _victim
            (:`Is Valid`
              (`AbilityTask_WaitGameplayEvent.WaitGameplayEvent` (struct :`TagName` "Event.Montage.FireBolt") null
                (:`EventReceived`
                  (bind _returnvalue_2 (`self.CalculateDamage`))
                  (`AbilitySystemComponent.BP_ApplyGameplayEffectSpecToSelf` (`AbilitySystemBlueprintLibrary.GetAbilitySystemComponent` _victim) _returnvalue_2))))
            (:`Is Not Valid`
              _)))))
    (:`Is Not Valid`
      _))
  (`self.K2_EndAbility`))