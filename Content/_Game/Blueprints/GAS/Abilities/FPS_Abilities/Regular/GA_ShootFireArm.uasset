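; Gameplay ability that fires the avatar's firearm through its combat component.
; On activation it binds a shoot-projectile delegate on the component, stops player sprinting, calls StartFiring, then immediately ends, which triggers StopFiring.
; The delegate callback spawns the projectile, prints debug text, and reports an AI noise event at the avatar's location unless the current weapon is suppressed.
; An invalid combat component logs an error and ends the ability.
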(event `self.K2_ActivateAbility`
  (bind _returnvalue (message `CombatInterface.GetCombatComponent` (`self.GetAvatarActorFromActorInfo`)))
  (`/Engine/EditorBlueprintResources/StandardMacros.IsValid` _returnvalue
    (:`Is Valid`
      (bind _output_get (set `self.CombatComponent` _returnvalue))
      (add `CombatComponent.ShootProjectileDelegate` _output_get (delegate `ShootProjectileDelegate_Event`))
      (`|ExecutionSequence`
        (:`then_0`
          (bind _asrpg_player_character (cast `RPG_Player_Character` (`self.GetAvatarActorFromActorInfo`)))
          (`/Engine/EditorBlueprintResources/StandardMacros.IsValid` _asrpg_player_character
            (:`Is Valid`
              (`RPG_Player_Character.StopSprinting` _asrpg_player_character))))
        (:`then_1`
          (`CombatComponent.StartFiring` (`self.CombatComponent`))
          (`self.K2_EndAbility`))))
    (:`Is Not Valid`
      (`|ExecutionSequence`
        (:`then_0`
          (`/Game/_Game/Blueprints/Libraries/BP_MicroLibrary.ErrorMessage` "COMBAT COMPONENT INVALID IN LMB ABILITY SHOOT"))
        (:`then_1`
          (`self.K2_EndAbility`))))))

(event `ShootProjectileDelegate_Event`
  (params (ProjectileClass :type "RPG_Projectile Class Reference") (MuzzleLocation :type "Vector Structure") (LaunchDirection :type "Rotator Structure"))
  (bind _returnvalue (`self.GetAvatarActorFromActorInfo`))
  (`self.SpawnProjectile` ProjectileClass MuzzleLocation LaunchDirection)
  (`KismetSystemLibrary.PrintString` "SHOOT PROJECTILE!" true true (struct :`R` 0.002694 :`G` 1.0 :`B` 0.065133 :`A` 1.0) 3.0 "1")
  (if (not (`.IsSupressed` (break `WeaponSettings` (`CombatComponent.CurrentWeaponSettings` (stale `self.K2_ActivateAbility` _output_get)))))
    (`AISense_Hearing.ReportNoiseEvent` (`Actor.K2_GetActorLocation` _returnvalue) 10.0 _returnvalue 5000.0)))

(event `self.K2_OnEndAbility`
  (params (bWasCancelled :type Boolean))
  (bind _combatcomponent (`self.CombatComponent`))
  (`/Engine/EditorBlueprintResources/StandardMacros.IsValid` _combatcomponent
    (:`Is Valid`
      (`CombatComponent.StopFiring` _combatcomponent))))