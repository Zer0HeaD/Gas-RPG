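; Gameplay ability for the IMP enemy's regular melee attack, gated by a shared attack token system.
; When one or no tokens remain, only the enemy closest to the player may try to reserve one from the tagged token actor.
; A successful reservation shows the attacking icon and runs a Combo Graph, simulating input on combo-end events for a randomized combo length.
; Graph end returns the token, hides the icon and ends the ability.
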(event `self.K2_ActivateAbility`
  ; Enemy Token System
  ;; Check if we got more than 1 available token. No reason for checking distance if 2 or more enemies got to attack
  (bind _incount (message `/Game/_Game/Blueprints/Interfaces/BPI_AIGroupInterface.GetMeleeTokenCount` (`self.FindTokenActor`)))
  (if (> _incount 1)
    ;; Assign token to enemy, proceed to attack
    (bind _success (message `/Game/_Game/Blueprints/Interfaces/BPI_AIGroupInterface.ReserveMeleeAttackToken` (`self.FindTokenActor`) 1 :!label _label))
    (if _success
      (message `/Game/_Game/Blueprints/Interfaces/BPI_AIGroupInterface.ShowAttackingIcon` (`self.GetAvatarActorFromActorInfo`))
      (set `self.CurrentCounter` 1)
      (set `self.Counter` (`KismetMathLibrary.RandomIntegerInRange` 1 (+ (`self.MaxCounter`) 1)))
      (bind (_asynctaskproxy _eventtag) (`ComboGraphAbilityTask_StartGraph.CreateStartComboGraph` "/Game/_Game/Blueprints/GAS/Abilities/SSH/RegularAttack/CG_IMP_RegularAttack.CG_IMP_RegularAttack" "/Game/_Game/Input/Actions/Combat/IA_RegularAttack.IA_RegularAttack" true)
        (:`OnGraphStart`
          (`/Engine/EditorBlueprintResources/StandardMacros.IncrementInt` (`self.CurrentCounter`)))
        (:`OnGraphEnd`
          (message `/Game/_Game/Blueprints/Interfaces/BPI_AIGroupInterface.ReturnMeleeAttackToken` (`self.FindTokenActor`) 1)
          (message `/Game/_Game/Blueprints/Interfaces/BPI_AIGroupInterface.HideAttackingIcon` (`self.GetAvatarActorFromActorInfo`))
          (`self.K2_EndAbility`))
        (:`EventReceived`
          (`|SwitchGameplayTag` _eventtag
            (:`Event.ComboGraph.Animation.ComboEnd`
              (if (<= (`self.CurrentCounter`) (`self.Counter`))
                (`/Engine/EditorBlueprintResources/StandardMacros.IncrementInt` (`self.CurrentCounter`)
                  (:`  `
                    (`ComboGraphBlueprintLibrary.SimulateComboInput` (`self.GetAvatarActorFromActorInfo`) "/Game/_Game/Input/Actions/Combat/IA_RegularAttack.IA_RegularAttack"))))))))
      (else
        (`self.K2_EndAbility`)))
    (else
      ;; Find closest enemy to player
      (bind _inenemy (message `/Game/_Game/Blueprints/Interfaces/BPI_AIGroupInterface.GetClosestEnemyToPlayer` (`self.FindTokenActor`)))
      (if (== _inenemy (`self.GetAvatarActorFromActorInfo`))
        (goto _label)
        (else
          (`self.K2_EndAbility`))))))

(fn `FindTokenActor`
  (returns (TokenActor :type "Actor Object Reference"))
  (locals (TokenActor_Local :type "Actor Object Reference"))
  (bind _outactors (`GameplayStatics.GetAllActorsWithTag` "TokenActor"))
  (for _array_element _outactors
    (set `local.TokenActor_Local` _array_element))
  (return (`local.TokenActor_Local`)))