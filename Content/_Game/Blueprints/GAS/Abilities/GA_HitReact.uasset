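; Gameplay ability that plays an avatar's hit reaction.
; On activation it applies GE_HitReact to the owner, gets the montage through the avatar's CombatInterface and plays it from a randomly picked section name.
; When the montage completes, is interrupted or is cancelled, it removes the effect by its stored handle and ends.
; An invalid interface only prints an error, leaving the effect applied and the ability not ended.
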(event `self.K2_ActivateAbility`
  (bind _returnvalue (`self.BP_ApplyGameplayEffectToOwner` "/Game/_Game/Blueprints/GAS/GameplayEffects/GE_HitReact.GE_HitReact_C"))
  (set `self.ActiveGA_HitReact` _returnvalue)
  (bind _ascombat_interface (cast `CombatInterface` (`self.GetAvatarActorFromActorInfo`))
    (:`then`
      (if (`KismetSystemLibrary.IsValidInterface` _ascombat_interface)
        (bind _returnvalue_2 (`CombatInterface.GetHitReactMontage` _ascombat_interface))
        (`AbilityTask_PlayMontageAndWait.CreatePlayMontageAndWaitProxy` "None" _returnvalue_2 1.0 (`KismetArrayLibrary.Array_Random` (`self.MontageSectionNames`))
          (:`OnCompleted`
            _)
          (:`OnInterrupted`
            _)
          (:`OnCancelled`
            _))
        (`self.BP_RemoveGameplayEffectFromOwnerWithHandle` (`self.ActiveGA_HitReact`))
        (`self.K2_EndAbility`)
        (else
          (`KismetSystemLibrary.PrintString` "HIT REACT ABILITY: INVALID INTERFACE!" true true (struct :`R` 1.0 :`B` 0.075939 :`A` 1.0) 10.0 :!label _label))))
    (:`CastFailed`
      (goto _label))))