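; Gameplay ability that makes an enemy perform a regular attack combo of random length.
; On activation it rolls a random attack count and starts the regular-attack Combo Graph.
; Each Combo End event from the graph simulates the attack input on the avatar until the count is reached, so the AI chains attacks like a player.
; The ability ends when the graph ends.
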(event `self.K2_ActivateAbility`
  (set `self.CurrentCounter` 1)
  (set `self.Counter` (`KismetMathLibrary.RandomIntegerInRange` 1 5))
  (bind (_asynctaskproxy _eventtag) (`ComboGraphAbilityTask_StartGraph.CreateStartComboGraph` "/Game/_Game/Blueprints/GAS/Abilities/SSH/RegularAttack/CG_SSH_RegularAttack.CG_SSH_RegularAttack" "/Game/_Game/Input/Actions/Combat/IA_RegularAttack.IA_RegularAttack" true)
    (:`OnGraphStart`
      (`/Engine/EditorBlueprintResources/StandardMacros.IncrementInt` (`self.CurrentCounter`)))
    (:`OnGraphEnd`
      (`self.K2_EndAbility`))
    (:`EventReceived`
      (`|SwitchGameplayTag` _eventtag
        (:`Event.ComboGraph.Animation.ComboEnd`
          (if (<= (`self.CurrentCounter`) (`self.Counter`))
            (`/Engine/EditorBlueprintResources/StandardMacros.IncrementInt` (`self.CurrentCounter`)
              (:`  `
                (`ComboGraphBlueprintLibrary.SimulateComboInput` (`self.GetAvatarActorFromActorInfo`) "/Game/_Game/Input/Actions/Combat/IA_RegularAttack.IA_RegularAttack")))))))))