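; Anim notify that restores the RPG player character's state at points during mantle and vault montages.
; A notify type setting picks one action: reset capsule radius, restore Pawn collision on capsule and mesh, switch to walking, or stop the montage.
; Other types restore controller yaw toward the obstacle rotation, or re-enable IK and quick-unholster the weapon through the combat component.
; The displayed notify name follows the selected type.
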(fn `GetNotifyName`
  (returns (ReturnValue :type String))
  (return (select `/Game/_Game/Blueprints/Enums/E_VM_NotifyType` (`self.NotifyType`) :`NewEnumerator0` "Switch Movement" :`NewEnumerator1` "Reset Collision" :`NewEnumerator2` "Reset Radius" :`NewEnumerator3` "Stop" :`NewEnumerator4` "Reset Controller" :`NewEnumerator5` "Unholster")))

(fn `Received_Notify`
  (params (MeshComp :type "SkeletalMeshComponent Object Reference") (Animation :type "AnimSequenceBase Object Reference") (EventReference :type "AnimNotifyEventReference Structure (by ref)"))
  (returns (ReturnValue :type Boolean))
  (bind _asbp_rpg_player_character (cast `/Game/_Game/Blueprints/Character/Player/BP_RPG_PlayerCharacter` (`ActorComponent.GetOwner` MeshComp)))
  (`/Engine/EditorBlueprintResources/StandardMacros.IsValid` _asbp_rpg_player_character
    (:`Is Valid`
      (if (`|EnumEquality` (`self.NotifyType`) "NewEnumerator2")
        (`CapsuleComponent.SetCapsuleRadius` (`Character.CapsuleComponent` _asbp_rpg_player_character) (`/Game/_Game/Blueprints/Character/Player/BP_RPG_PlayerCharacter.Original Capsule Radius` _asbp_rpg_player_character) true)
        (return true)
        (elif (`|EnumEquality` (`self.NotifyType`) "NewEnumerator1")
          (`PrimitiveComponent.SetCollisionObjectType` (`Character.CapsuleComponent` _asbp_rpg_player_character) "ECC_Pawn")
          (`PrimitiveComponent.SetCollisionObjectType` (`Character.Mesh` _asbp_rpg_player_character) "ECC_Pawn")
          (return true)
          (elif (`|EnumEquality` (`self.NotifyType`) "NewEnumerator0")
            (`CharacterMovementComponent.SetMovementMode` (`Character.CharacterMovement` _asbp_rpg_player_character) "MOVE_Walking" 0)
            (return true)
            (elif (`|EnumEquality` (`self.NotifyType`) "NewEnumerator3")
              (`Character.StopAnimMontage` _asbp_rpg_player_character (`Character.GetCurrentMontage` _asbp_rpg_player_character))
              (return true)
              (elif (`|EnumEquality` (`self.NotifyType`) "NewEnumerator4")
                (set `/Game/_Game/Blueprints/Character/Player/BP_RPG_PlayerCharacter.InVaultMantle` false _asbp_rpg_player_character)
                (set `Pawn.bUseControllerRotationYaw` true _asbp_rpg_player_character)
                (`Controller.SetControlRotation` (`GameplayStatics.GetPlayerController` 0) (`/Game/_Game/Blueprints/Character/Player/BP_RPG_PlayerCharacter.FinalRotationTowardsObstacle` _asbp_rpg_player_character))
                (set `/Game/_Game/Blueprints/Character/Player/BP_RPG_PlayerCharacter.FinalRotationTowardsObstacle` (struct) _asbp_rpg_player_character)
                (return true)
                (elif (`|EnumEquality` (`self.NotifyType`) "NewEnumerator5")
                  (set `/Game/_Game/Blueprints/Character/Player/BP_RPG_PlayerCharacter.DisableRightHandIK` false _asbp_rpg_player_character)
                  (`CombatComponent.QuickUnholsterWeapon` (`RPG_Player_Character.CombatComponent` _asbp_rpg_player_character) false)
                  (set `/Game/_Game/Blueprints/Character/Player/BP_RPG_PlayerCharacter.DisableBodyControlIK` false _asbp_rpg_player_character)
                  (return true))))))))))