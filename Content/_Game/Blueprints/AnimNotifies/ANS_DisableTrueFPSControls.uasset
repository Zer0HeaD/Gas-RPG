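; Anim notify state that marks the window of a full-body animation on the first-person player, going by its name to disable true-FPS controls.
; On begin it sets IsFullBodyMotion on the ABP_FPS_Player anim instance, and on end it clears that flag.
; On end it also gets the owner's combat component, sets the player state to Unoccupied and reattaches the current weapon to SOCKET_Weapon.
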(fn `Received_NotifyBegin`
  (params (MeshComp :type "SkeletalMeshComponent Object Reference") (Animation :type "AnimSequenceBase Object Reference") (TotalDuration :type "Float (single-precision)") (EventReference :type "AnimNotifyEventReference Structure (by ref)"))
  (returns (ReturnValue :type Boolean))
  (bind _asabp_fps_player (cast `/Game/_Game/Blueprints/Character/Animations/ABP_FPS_Player` (`SkeletalMeshComponent.GetAnimInstance` MeshComp)))
  (`/Engine/EditorBlueprintResources/StandardMacros.IsValid` _asabp_fps_player
    (:`Is Valid`
      (set `/Game/_Game/Blueprints/Character/Animations/ABP_FPS_Player.IsFullBodyMotion` true _asabp_fps_player)
      (return true))
    (:`Is Not Valid`
      (`|ExecutionSequence`
        (:`then_0`
          (`/Game/_Game/Blueprints/Libraries/BP_MicroLibrary.ErrorMessage` "INVALID CAST TO ANIM INSTANCE ON BEGIN!"))
        (:`then_1`
          (return false))))))

(fn `Received_NotifyEnd`
  (params (MeshComp :type "SkeletalMeshComponent Object Reference") (Animation :type "AnimSequenceBase Object Reference") (EventReference :type "AnimNotifyEventReference Structure (by ref)"))
  (returns (ReturnValue :type Boolean))
  (bind _asabp_fps_player (cast `/Game/_Game/Blueprints/Character/Animations/ABP_FPS_Player` (`SkeletalMeshComponent.GetAnimInstance` MeshComp)))
  (`/Engine/EditorBlueprintResources/StandardMacros.IsValid` _asabp_fps_player
    (:`Is Valid`
      (set `/Game/_Game/Blueprints/Character/Animations/ABP_FPS_Player.IsFullBodyMotion` false _asabp_fps_player)
      (bind _returnvalue (message `CombatInterface.GetCombatComponent` (`ActorComponent.GetOwner` MeshComp)))
      (`/Engine/EditorBlueprintResources/StandardMacros.IsValid` _returnvalue
        (:`Is Valid`
          (`CombatComponent.SetPlayerState` _returnvalue "Unoccupied")
          (`CombatComponent.AttachCurrentWeaponToSocket` _returnvalue "SOCKET_Weapon")
          (return true))
        (:`Is Not Valid`
          (`|ExecutionSequence`
            (:`then_0`
              (`/Game/_Game/Blueprints/Libraries/BP_MicroLibrary.ErrorMessage` "OWNER DON'T HAVE A COMBAT COMPONENT!"))
            (:`then_1`
              (return false))))))
    (:`Is Not Valid`
      (`|ExecutionSequence`
        (:`then_0`
          (`/Game/_Game/Blueprints/Libraries/BP_MicroLibrary.ErrorMessage` "INVALID CAST TO ANIM INSTANCE ON END!"))
        (:`then_1`
          (return false))))))