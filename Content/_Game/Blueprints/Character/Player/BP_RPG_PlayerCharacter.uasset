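; Player character Blueprint for the RPG that toggles between explore and combat stances for magic staff locomotion.
; Left Alt flip-flops the locomotion component's animset and rotation mode, with controller yaw rotation off in explore and on in combat.
; A helper prints orange debug text, while unconnected nodes hold compass, ability system debug and example UI snippets.
; BeginPlay and the construction script are empty.
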(event `self.ReceiveBeginPlay`)

(event `Key|LeftAlt`
  (params (Key :type "Key Structure"))
  (bind _ct_cmpt_locomotion (`self.CT_Cmpt_Locomotion`))
  (:`Pressed`
    (`/Engine/EditorBlueprintResources/StandardMacros.FlipFlop`
      (:`A`
        (`/Game/LocomotionSystem/Assets/CT_Components/LocomotionSystem/Components/CT_Cmpt_Locomotion.SetAnimset` _ct_cmpt_locomotion "MagicStaff_Explore")
        (`/Game/LocomotionSystem/Assets/CT_Components/LocomotionSystem/Components/CT_Cmpt_Locomotion.SetRotationMode` _ct_cmpt_locomotion "NewEnumerator1")
        (set `self.bUseControllerRotationYaw` false))
      (:`B`
        (`/Game/LocomotionSystem/Assets/CT_Components/LocomotionSystem/Components/CT_Cmpt_Locomotion.SetAnimset` _ct_cmpt_locomotion "MagicStaff_Combat")
        (`/Game/LocomotionSystem/Assets/CT_Components/LocomotionSystem/Components/CT_Cmpt_Locomotion.SetRotationMode` _ct_cmpt_locomotion "NewEnumerator0")
        (set `self.bUseControllerRotationYaw` true)))))

(fn `UserConstructionScript`)