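; Archer enemy Blueprint that equips a bow and drives its arrow sequence, extending a parent's BeginPlay and construction logic.
; On BeginPlay it spawns a BP_Demo_Bow, stores the reference and snaps it to the mesh's Bow_Socket.
; Three custom events forward to the bow to make, connect and fire the arrow.
; The make-arrow event also sets the movement type on the locomotion component.
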(event `self.ReceiveBeginPlay`
  (`parent.ReceiveBeginPlay`)
  (bind _returnvalue (`|SpawnActorFromClass` "/Game/Demo_Archer/Bow/BP_Demo_Bow.BP_Demo_Bow_C" (`KismetMathLibrary.MakeTransform` (0.0 0.0 0.0)) "Undefined" "MultiplyWithRoot" self null))
  (bind _output_get (set `self.Bow` _returnvalue))
  (`self.K2_AttachToComponent` _output_get (`self.Mesh`) "Bow_Socket" "SnapToTarget" "SnapToTarget" "KeepRelative" true))

(event `/Game/_Game/Blueprints/Interfaces/BPI_AI_Interface.Archer_MakeArrow`
  (`/Game/LocomotionSystem/Assets/CT_Components/LocomotionSystem/Components/CT_Cmpt_Locomotion.SetMovementType` (`self.CT_Cmpt_Locomotion`) "NewEnumerator0")
  (`/Game/Demo_Archer/Bow/BP_Demo_Bow.MakeArrow` (`self.Bow`)))

(event `/Game/_Game/Blueprints/Interfaces/BPI_AI_Interface.Archer_Draw`
  (`/Game/Demo_Archer/Bow/BP_Demo_Bow.ConnectArrow` (`self.Bow`)))

(event `/Game/_Game/Blueprints/Interfaces/BPI_AI_Interface.Archer_DeleteFakeArrow`
  (`/Game/Demo_Archer/Bow/BP_Demo_Bow.FireArrow` (`self.Bow`)))

(fn `UserConstructionScript`
  (`parent.UserConstructionScript`))