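; Player controller for the RPG that caches its controlled RPG_Player_Character on BeginPlay and holds logic for a gamepad-driven UI cursor.
; CursorFollowController moves the mouse by IA_Move input, scaled by gamepad sensitivity and delta time, when a gamepad is the latest device, printing the position for debugging.
; Its only call, gated on the character's UIOpened flag, is disconnected from the empty Tick, so the cursor logic never runs.
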(event `self.ReceiveBeginPlay`
  (bind _asrpg_player_character (cast `RPG_Player_Character` (`self.K2_GetPawn`)))
  (`/Engine/EditorBlueprintResources/StandardMacros.IsValid` _asrpg_player_character
    (:`Is Valid`
      (set `self.As RPG Player Character` _asrpg_player_character))))

(event `self.ReceiveTick`
  (params (DeltaSeconds :type "Float (single-precision)")))

(fn `CursorFollowController`
  (params (deltaTime :type "Float (double-precision)"))
  (bind (_locationx _locationy) (`self.GetMousePosition`))
  (bind (_returnvalue_x _returnvalue_y) (`KismetMathLibrary.BreakVector2D` (`|GetInputActionValue`)))
  (bind (_returnvalue_x_2 _returnvalue_y_2) (`KismetMathLibrary.BreakVector2D` (`|GetInputActionValue`)))
  (bind (_returnvalue_inputclassname _returnvalue_hardwaredeviceidentifier _returnvalue_primarydevicetype) (break `HardwareDeviceIdentifier` (`InputDeviceSubsystem.GetMostRecentlyUsedHardwareDevice` :`self` (subsystem `InputDeviceSubsystem`))))
  (bind (_returnvalue_x_3 _returnvalue_y_3) (`KismetMathLibrary.BreakVector2D` (`KismetMathLibrary.MakeVector2D` _locationx _locationy)))
  (bind (_returnvalue_x_4 _returnvalue_y_4) (`KismetMathLibrary.BreakVector2D` (+ (`KismetMathLibrary.MakeVector2D` _returnvalue_x_3 _returnvalue_y_3) (* (* (`KismetMathLibrary.MakeVector2D` _returnvalue_x_2 (* _returnvalue_y_2 -1.0)) (`self.UI_SensitivityGamepad`)) (`local.deltaTime`)))))
  (bind _returnvalue (`KismetMathLibrary.FTrunc` _returnvalue_x_4))
  (bind _returnvalue_2 (`KismetMathLibrary.FTrunc` _returnvalue_y_4))
  (if (`|EnumEquality` _returnvalue_primarydevicetype "Gamepad")
    (if (or (> (`KismetMathLibrary.Abs` _returnvalue_x) 0.0) (> (`KismetMathLibrary.Abs` _returnvalue_y) 0.0))
      (`self.SetMouseLocation` _returnvalue _returnvalue_2)
      (`KismetSystemLibrary.PrintString` (`KismetTextLibrary.Conv_TextToString` (`|FormatText` "x{x} y{y}" _returnvalue _returnvalue_2)) true true (struct :`G` 0.66 :`B` 1.0 :`A` 1.0) 2.0 "0"))))

(fn `UserConstructionScript`)