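; AI controller for RPG enemies that drives a detection meter and mirrors enemy state enums and target locations into the Blackboard.
; Perception updates feed Handle Sight, though the check passes the Damage sense; hearing's investigation response is disconnected.
; Detection raises a meter widget with a sound, and Tick updates the level.
; Looping timers switch the human state to Investigating or Attacking at thresholds; losing the player while attacking switches to Searching.
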(event OnPerceptionUpdated(AIPerception)
  (params (UpdatedActors :type Array%20of%20Actor%20Object%20References))
  (for _array_element UpdatedActors
    (Utilities|FlowControl|Sequence
      (:then_0
        (bind _success (CallFunction|CanSensePlayer _array_element "NewEnumerator3"))
        (if _success
          (|HandleSight _array_element :!label _label)
          (else
            (goto _label False))))
      (:then_1
        (bind (_success_2 _stimulus) (CallFunction|CanSensePlayer _array_element "NewEnumerator2")))
      (:then_2
        (bind _success_3 (CallFunction|CanSensePlayer _array_element "NewEnumerator3"))
        (if _success_3
          (Development|PrintString "damaged"))))))

(event OnTargetPerceptionForgotten(AIPerception)
  (params (Actor :type Actor%20Object%20Reference)))

(event OnTargetPerceptionUpdated(AIPerception)
  (params (Actor :type Actor%20Object%20Reference) (Stimulus :type AI%20Stimulus%20Structure))
  (Utilities|SwitchonHumanState
    (:Detecting
      (if (or (== Actor (Game|GetPlayerCharacter 0)) (Actor|ActorHasTag Actor "UpperBodyStimulus"))
        (AI|Components|Blackboard|SetValueasVector (AI|GetBlackboard 0) (Variables|BlackboardNames|GetDetection%20Point%20Key%20Name) (.StimulusLocation (Utilities|Struct|BreakAIStimulus Stimulus)))))))

(event EventBeginPlay
  (Utilities|FlowControl|Sequence
    (:then_0
      (bind _asbp_rpg_enemy_base (Utilities|Casting|CastToBP_RPG_Enemy_Base (Pawn|GetControlledPawn)))
      (Utilities|IsValid _asbp_rpg_enemy_base
        (:Is%20Valid
          (Variables|Default|SetAs%20BP%20RPG%20Enemy%20Base _asbp_rpg_enemy_base))))
    (:then_1
      (Variables|Default|GetAs%20BP%20RPG%20Enemy%20Base
        (:then
          (AI|Components|Blackboard|SetValueasEnum (AI|GetBlackboard 0) (Variables|BlackboardNames|GetState%20Key%20Name) (Variables|/Game/_Game/Blueprints/Character/Enemies/BP_RPG_Enemy_Base.BP_RPG_Enemy_Base_C|GetState (Variables|Default|GetAs%20BP%20RPG%20Enemy%20Base)))
          (AI|Components|Blackboard|SetValueasEnum (AI|GetBlackboard 0) (Variables|BlackboardNames|GetHuman%20State%20Key%20Name) (Variables|/Game/_Game/Blueprints/Character/Enemies/BP_RPG_Enemy_Base.BP_RPG_Enemy_Base_C|GetHumanState (Variables|Default|GetAs%20BP%20RPG%20Enemy%20Base)))
          (AI|Components|Blackboard|SetValueasEnum (AI|GetBlackboard 0) (Variables|BlackboardNames|GetSearching%20State%20Key%20Name) (Variables|/Game/_Game/Blueprints/Character/Enemies/BP_RPG_Enemy_Base.BP_RPG_Enemy_Base_C|GetSearchingState (Variables|Default|GetAs%20BP%20RPG%20Enemy%20Base))))
        (:else)))))

(event EventTick
  (params (DeltaSeconds :type Float%20%28single-precision%29))
  (Utilities|FlowControl|Sequence
    (:then_0
      (if (Variables|Default|GetDetectPlayer)
        (Variables|Default|SetDetectionLevel (|IncreaseDetectionLevel))
        (else
          (bind _output_get (Variables|Default|SetDetectionLevel (|DecreaseDetectionLevel))))))
    (:then_1
      (Development|PrintString (Utilities|String|ToString(Text) (Utilities|Text|FormatText "Detection level {dl}" (Variables|Default|GetDetectionLevel))) true true "(R=1.000000,G=0.350000,B=0.050000,A=1.000000)" 0.0)
      (CallFunction|UpdateDetectionPercent))))

(event EventSetSearchingStateInterface
  (params (NewState :type E_SearchingState%20Enum :default "NewEnumerator0"))
  (CallFunction|SetSearchingState NewState))

(event EventSetTargetCoverLocation
  (params (NewTargetCoverLocation :type Vector :default "0, 0, 0"))
  (AI|Components|Blackboard|SetValueasVector (AI|GetBlackboard 0) (Variables|BlackboardNames|GetTarget%20Cover%20Location%20Point%20Key%20Name) NewTargetCoverLocation))

(fn ConstructionScript)

(fn CanSensePlayer
  (params (Actor :type Actor%20Object%20Reference) (Sense :type E_AISense%20Enum :default "NewEnumerator0"))
  (bind _info (Class|AIPerceptionComponent|GetActorsPerception (Variables|Default|GetAIPerception) Actor))
  (for _array_element (.LastSensedStimuli (Utilities|Struct|BreakActorPerceptionBlueprintInfo _info))
    (bind _returnvalue (Class|AIPerceptionSystem|GetSenseClassforStimulus _array_element))
    (if (and (== _returnvalue (Utilities|Select :Index Sense :NewEnumerator0 0 :NewEnumerator1 "/Script/AIModule.AISense_Sight" :NewEnumerator2 "/Script/AIModule.AISense_Hearing" :NewEnumerator3 "/Script/AIModule.AISense_Damage")) (or (== (.Target (Utilities|Struct|BreakActorPerceptionBlueprintInfo _info)) (Game|GetPlayerCharacter 0)) (Actor|ActorHasTag (.Target (Utilities|Struct|BreakActorPerceptionBlueprintInfo _info)) "UpperBodyStimulus")))
      (return (.bSuccessfullySensed (Utilities|Struct|BreakAIStimulus _array_element)) _array_element))))

(fn SetHumanState
  (params (NewState :type E_SA_HumanState%20Enum :default "NewEnumerator0"))
  (bind _as_bp_rpg_enemy_base (Variables|Default|GetAs%20BP%20RPG%20Enemy%20Base)
    (:then
      (bind _output_get (Variables|/Game/_Game/Blueprints/Character/Enemies/BP_RPG_Enemy_Base.BP_RPG_Enemy_Base_C|SetHumanState _as_bp_rpg_enemy_base NewState))
      (AI|Components|Blackboard|SetValueasEnum (AI|GetBlackboard 0) (Variables|BlackboardNames|GetHuman%20State%20Key%20Name) _output_get)
      (return))
    (:else)))

(fn HandleonSight)

(fn CreateDetectionWidget
  (bind _returnvalue (UserInterface|CreateWidget "/Game/_Game/Blueprints/UI/WBP_DetectionWidget.WBP_DetectionWidget_C" (Game|GetPlayerController 0)))
  (bind _output_get (Variables|Default|SetDetectionWidget _returnvalue))
  (Variables|/Game/_Game/Blueprints/UI/WBP_DetectionWidget.WBP_DetectionWidget_C|SetDetectorActor _output_get self)
  (UserInterface|Viewport|AddtoViewport _output_get 0)
  (return))

(fn RemoveDetectionWidget
  (Utilities|IsValid (Variables|Default|GetDetectionWidget)
    (:Is%20Valid
      (Widget|RemovefromParent (Variables|Default|GetDetectionWidget))
      (Variables|Default|SetDetectionWidget 0))))

(fn UpdateDetectionPercent
  (bind _detectionwidget (Variables|Default|GetDetectionWidget))
  (Utilities|IsValid _detectionwidget
    (:Is%20Valid
      (Variables|/Script/UMG.ProgressBar|SetPercent (Variables|/Game/_Game/Blueprints/UI/WBP_DetectionWidget.WBP_DetectionWidget_C|GetProgressBar_Detection _detectionwidget) (/ (Variables|Default|GetDetectionLevel) (Variables|Default|GetMaxDetectionLevel))))))

(fn SetSearchingState
  (params (NewState :type E_SearchingState%20Enum :default "NewEnumerator0"))
  (bind _as_bp_rpg_enemy_base (Variables|Default|GetAs%20BP%20RPG%20Enemy%20Base)
    (:then
      (bind _output_get (Variables|/Game/_Game/Blueprints/Character/Enemies/BP_RPG_Enemy_Base.BP_RPG_Enemy_Base_C|SetSearchingState _as_bp_rpg_enemy_base NewState))
      (AI|Components|Blackboard|SetValueasEnum (AI|GetBlackboard 0) (Variables|BlackboardNames|GetSearching%20State%20Key%20Name) _output_get)
      (return))
    (:else)))

(event Custom|Handle%20Remove%20Detection%20Widget
  (bind _detectionlevel (Variables|Default|GetDetectionLevel))
  ;[0.15 0.15 0.15 0.5] Create Detection Widget And Handle Removing
  (if (or (<= _detectionlevel 0.0) (>= _detectionlevel 1e+02))
    (CallFunction|RemoveDetectionWidget)
    (Utilities|Time|ClearandInvalidateTimerbyHandle (Variables|Default|GetRemoveDetectionWidget_TimerHandle))))

(event Custom|Check%20To%20Start%20Investigating
  (|CheckToStartInvestigate (stale _actor)))

(event Custom|Check%20To%20Start%20Attacking
  (|CheckToStartAttack))