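; BP_ItemBase is a base pickup item whose PickupItem event applies an instant Gameplay Effect to the player character and plays a sound at the item's location.
; OnPickupItem calls a step that interpolates the item's rotation and location toward just above the player, then clears the timer and destroys it when close.
; The collision disable and per-frame looping timer meant to drive that homing motion are disconnected, so they never run.
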(event `self.ReceiveTick`
  (params (DeltaSeconds :type "Float (single-precision)")))

(event `Pickup Item`
  (`self.ApplyEffectToTarget` (`GameplayStatics.GetPlayerCharacter` 0) (`self.InstantGameplayEffectClass`))
  (`GameplayStatics.PlaySoundAtLocation` (`self.Pickup Sound`) (`self.K2_GetActorLocation`) (struct) 1.0 1.0 0.0 null null null null))

(event `On Pickup Item`
  (bind _returnvalue (`self.K2_GetActorLocation`))
  (bind _returnvalue_2 (+ (`self.K2_GetActorLocation` (`GameplayStatics.GetPlayerCharacter` 0)) (0.0 0.0 35.0)))
  (`self.K2_SetActorRotation` (`KismetMathLibrary.RInterpTo` (`self.K2_GetActorRotation`) (`KismetMathLibrary.FindLookAtRotation` (`self.K2_GetActorLocation`) (`self.K2_GetActorLocation` (`GameplayStatics.GetPlayerCharacter` 0))) (`GameplayStatics.GetWorldDeltaSeconds`) 10.0))
  (`self.K2_SetActorLocation` (`KismetMathLibrary.VInterpTo` _returnvalue _returnvalue_2 (`GameplayStatics.GetWorldDeltaSeconds`) 7.0))
  (if (< (`KismetMathLibrary.Vector_Distance` _returnvalue _returnvalue_2) 25.0)
    (`KismetSystemLibrary.K2_ClearAndInvalidateTimerHandle` (`self.PickupItem_TimerHandle`))
    (`self.K2_DestroyActor`)))

(fn `UserConstructionScript`)