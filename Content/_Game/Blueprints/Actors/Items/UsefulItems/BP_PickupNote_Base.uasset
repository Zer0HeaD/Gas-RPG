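; BP_PickupNote_Base is a base pickup note actor that opens and closes a readable note when the player completes an interaction.
; A FlipFlop on the interaction component toggles between the two states.
; Opening applies an instant gameplay effect to the player, shows the note widget with mouse input, switches HUD display and slows global time.
; Closing animates the widget away and restores game input, HUD and normal time.
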(event `self.ReceiveBeginPlay`
  (`parent.ReceiveBeginPlay`))

(event `self.InteractionComponent.OnInteractionCompleted`
  (bind _returnvalue (`GameplayStatics.GetPlayerController` 0))
  (bind _shooterhudmanager (`/Game/CompShooterHUD/Blueprints/Interfaces/FL_ShooterHud.GetShooterHudManager`))
  (`/Engine/EditorBlueprintResources/StandardMacros.FlipFlop`
    (:`A`
      (`self.ApplyEffectToTarget` (`GameplayStatics.GetPlayerCharacter` 0) (`self.InstantGameplayEffectClass`))
      (`GameplayStatics.PlaySound2D` (`self.Pickup Sound`) 1.0 1.0 0.0 null null)
      (bind _returnvalue_2 (`|CreateWidget` "/Game/_Game/Blueprints/UI/NoteWidget/WBP_NoteBase.WBP_NoteBase_C" _returnvalue))
      (bind _output_get (set `self.NoteWidget` _returnvalue_2))
      (`UserWidget.AddToViewport` _output_get 0)
      (`WidgetBlueprintLibrary.SetInputMode_GameAndUIEx` _returnvalue _output_get "LockInFullscreen" false)
      (set `PlayerController.bShowMouseCursor` true _returnvalue)
      (`/Game/ProHUDV2/Blueprints/Libraries/BPi_HUDManagerV2.HideHUD` (`/Game/ProHUDV2/Blueprints/Libraries/BP_PHV2_Functions.GetHUDManager`))
      (`/Game/CompShooterHUD/Blueprints/Interfaces/I_ShooterHudManager.DisplayShooterHUD` _shooterhudmanager "NewEnumerator1" 1)
      (`GameplayStatics.SetGlobalTimeDilation` 0.1))
    (:`B`
      (`self.NoteWidget`
        (:`then`
          (`GameplayStatics.PlaySound2D` (`self.CloseSound`) 1.0 1.0 0.0 null null)
          (`/Game/_Game/Blueprints/UI/NoteWidget/WBP_NoteBase.CloseWidgetWithAnimation` (`self.NoteWidget`))
          (`WidgetBlueprintLibrary.SetInputMode_GameOnly` _returnvalue)
          (set `PlayerController.bShowMouseCursor` false _returnvalue)
          (`/Game/ProHUDV2/Blueprints/Libraries/BPi_HUDManagerV2.ShowHUD` (`/Game/ProHUDV2/Blueprints/Libraries/BP_PHV2_Functions.GetHUDManager`))
          (`/Game/CompShooterHUD/Blueprints/Interfaces/I_ShooterHudManager.DisplayShooterHUD` _shooterhudmanager "NewEnumerator0" 1)
          (`GameplayStatics.SetGlobalTimeDilation` 1.0))
        (:`else`)))))

(fn `UserConstructionScript`
  (`parent.UserConstructionScript`))