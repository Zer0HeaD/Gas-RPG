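; Base actor for ammo pickups that give the player ammo of a set type and amount through an interaction.
; When the interaction completes, it compares current and max ammo for that type in the player character's combat component.
; At max, it only changes the interaction component's finish method.
; Otherwise it sets a different finish method, adds the ammo, updates the weapon bar and picks up the item.
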(event `Check If Can Pickup Event`
  (bind _interactioncomponent (`self.InteractionComponent`))
  (bind _returnvalue (message `CombatInterface.GetCombatComponent` (`GameplayStatics.GetPlayerCharacter` 0)))
  (`/Engine/EditorBlueprintResources/StandardMacros.IsValid` _returnvalue
    (:`Is Valid`
      (bind (_currentammo _maxammo) (break `AmmoData` (`BlueprintMapLibrary.Map_Find` (`CombatComponent.AmmoMap` _returnvalue) (`self.AmmoType`))))
      (if (== _currentammo _maxammo)
        (`/Game/InteractionEssentials/Blueprints/Components/InteractionComponent.Set_InteractionFinishMethod` _interactioncomponent "NewEnumerator2")
        (else
          (`/Game/InteractionEssentials/Blueprints/Components/InteractionComponent.Set_InteractionFinishMethod` _interactioncomponent "NewEnumerator0")
          (`CombatComponent.AddAmmo` _returnvalue (`self.AmmoType`) (`self.AmmoToAdd`))
          (message `/Game/_Game/Blueprints/Interfaces/BPI_PlayerCharacterUtility.Update Weapon Bar Ammo` (`GameplayStatics.GetPlayerCharacter` 0))
          (`self.Pickup Item`))))))

(event `self.InteractionComponent.OnInteractionCompleted`
  (`self.Check If Can Pickup Event`))

(fn `UserConstructionScript`
  (`parent.UserConstructionScript`))