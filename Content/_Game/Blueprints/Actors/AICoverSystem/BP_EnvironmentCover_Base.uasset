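; Base environment cover actor for the AI cover system, which enemies investigate while searching.
; When the assigned enemy enters the sphere of a reserved, uninvestigated cover, it writes the farther of two billboard side points to the blackboard.
; It then advances the AI's searching state, marks the cover investigated and updates a debug status widget.
; A looping timer can blink overlap generation to retrigger detection, and is cleared on success.
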(event `self.ReceiveBeginPlay`
  (`KismetSystemLibrary.Delay` 0.2)
  (`self.Set Text In Widget` false))

(event `self.CoverSphereCollision.OnComponentBeginOverlap`
  (params (OverlappedComponent :type "PrimitiveComponent Object Reference") (OtherActor :type "Actor Object Reference") (OtherComp :type "PrimitiveComponent Object Reference") (OtherBodyIndex :type Integer) (bFromSweep :type Boolean) (SweepResult :type "HitResult Structure (by ref)"))
  (bind _returnvalue (`AIBlueprintHelperLibrary.GetAIController` OtherActor))
  (bind (_coverstatus_bisreserved _coverstatus_bisinvestigated _coverstatus_assignedaicharacter) (break `/Game/_Game/Blueprints/Structs/F_CoverStruct` (`self.CoverStatus`)))
  (if (`self.ActorHasTag` OtherActor "Human")
    (bind _asbp_rpg_ai_controller (cast `/Game/_Game/Blueprints/AI/BP_RPG_AI_Controller` _returnvalue))
    (bind _inawarnedstate (message `/Game/_Game/Blueprints/Interfaces/BPI_AIController_Interface.GetAwarnedState` _returnvalue))
    (switch `/Game/_Game/Blueprints/Enums/E_AwarnedStates` _inawarnedstate
      (:`NewEnumerator0`
        (bind _asbp_rpg_enemy_base (cast `/Game/_Game/Blueprints/Character/Enemies/BP_RPG_Enemy_Base` (`Controller.K2_GetPawn` _asbp_rpg_ai_controller)))
        (`/Engine/EditorBlueprintResources/StandardMacros.IsValid` _asbp_rpg_enemy_base
          (:`Is Valid`
            (if (and (== _asbp_rpg_enemy_base _coverstatus_assignedaicharacter) _coverstatus_bisreserved (not _coverstatus_bisinvestigated))
              (`KismetSystemLibrary.K2_ClearAndInvalidateTimerHandle` (`self.RetriggerOverlapEvent_TimerHandle`))
              (`|ExecutionSequence`
                (:`then_0`
                  (if (>= (`KismetMathLibrary.Vector_Distance` (`SceneComponent.K2_GetComponentLocation` (`self.Billboard_01`)) (`self.K2_GetActorLocation` OtherActor)) (`KismetMathLibrary.Vector_Distance` (`SceneComponent.K2_GetComponentLocation` (`self.Billboard_02`)) (`self.K2_GetActorLocation` OtherActor)))
                    (set `self.TargetCoverSidePoint` (`SceneComponent.K2_GetComponentLocation` (`self.Billboard_01`)))
                    (else
                      (set `self.TargetCoverSidePoint` (`SceneComponent.K2_GetComponentLocation` (`self.Billboard_02`))))))
                (:`then_1`
                  (`BlackboardComponent.SetValueAsVector` (`AIBlueprintHelperLibrary.GetBlackboard` _asbp_rpg_ai_controller) (`self.Target Cover Side Point Key Name`) (`self.TargetCoverSidePoint`))
                  (`/Game/_Game/Blueprints/AI/BP_RPG_AI_Controller.SetSearchingState` _asbp_rpg_ai_controller "NewEnumerator2")
                  (bind _output_get (set `self.CoverStatus` (make `/Game/_Game/Blueprints/Structs/F_CoverStruct` true true)))
                  (bind (_bisreserved _bisinvestigated) (break `/Game/_Game/Blueprints/Structs/F_CoverStruct` _output_get))
                  (`self.Set Text In Widget` _bisreserved _bisinvestigated)))
              (else
                (`KismetSystemLibrary.PrintString` "WARNING! Another pawn who not assigned to this cover entered!")))))))))

(event `Set Text In Widget`
  (params (IsReserved :type Boolean) (IsInvestigated :type Boolean))
  ; Debug: Update Info about cover Status
  (bind _aswbp_cover_debug_widget (cast `/Game/_Game/Blueprints/UI/Debug_Widgets/WBP_CoverDebugWidget` (`WidgetComponent.GetWidget` (`self.TextWidget`))))
  (`/Engine/EditorBlueprintResources/StandardMacros.IsValid` _aswbp_cover_debug_widget
    (:`Is Valid`
      (`/Game/_Game/Blueprints/UI/Debug_Widgets/WBP_CoverDebugWidget.Set Text In Widget` _aswbp_cover_debug_widget (`|FormatText` "Is Reserved: {R},  \\n Is Invetigated {I}" IsReserved IsInvestigated)))))

(event `Retrigger Sphere Overlap`
  ; Blink collision on enemy state reaching it
  (bind _returnvalue (`KismetSystemLibrary.K2_SetTimerDelegate` (delegate `Retrigger Overlap event`) 0.5 true))
  (set `self.RetriggerOverlapEvent_TimerHandle` _returnvalue))

(event `Retrigger Overlap event`
  (bind _coverspherecollision (`self.CoverSphereCollision`))
  ; Blink collision on enemy state reaching it
  (set `PrimitiveComponent.bGenerateOverlapEvents` false _coverspherecollision)
  (`KismetSystemLibrary.RetriggerableDelay` 0.2)
  (set `PrimitiveComponent.bGenerateOverlapEvents` true _coverspherecollision))

(fn `UserConstructionScript`)