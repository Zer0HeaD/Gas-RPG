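; Area manager that coordinates human enemy AI searching environment covers.
; Its box, enabled after a short delay, registers overlapping covers and enemies.
; A looping timer polls AI controller states and, when search-ready, reserves the first free cover for the closest eligible enemy, sending that controller the location and new search state.
; A second timer clears cover statuses once all are investigated.
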(event `self.ReceiveBeginPlay`
  ; Initial enabling Collision with delay
  (`KismetSystemLibrary.Delay` 0.2)
  (`PrimitiveComponent.SetCollisionResponseToChannel` (`self.Box`) "ECC_GameTraceChannel9" "ECR_Overlap")
  (`PrimitiveComponent.SetCollisionResponseToChannel` (`self.Box`) "ECC_Pawn" "ECR_Overlap")
  (`self.Check if AI In Searching state`)
  (`self.Reset Covers`))

(event `self.ReceiveTick`
  (params (DeltaSeconds :type "Float (single-precision)")))

(event `self.Box.OnComponentBeginOverlap`
  (params (OverlappedComponent :type "PrimitiveComponent Object Reference") (OtherActor :type "Actor Object Reference") (OtherComp :type "PrimitiveComponent Object Reference") (OtherBodyIndex :type Integer) (bFromSweep :type Boolean) (SweepResult :type "HitResult Structure (by ref)"))
  (`|ExecutionSequence`
    (:`then_0`
      (if (`self.ActorHasTag` OtherActor "Cover")
        (bind _asbp_environment_cover_base (cast `/Game/_Game/Blueprints/Actors/AICoverSystem/BP_EnvironmentCover_Base` OtherActor))
        (`/Engine/EditorBlueprintResources/StandardMacros.IsValid` _asbp_environment_cover_base
          (:`Is Valid`
            (`KismetArrayLibrary.Array_AddUnique` (`self.CoverActors`) _asbp_environment_cover_base)))))
    (:`then_1`
      (if (`self.ActorHasTag` OtherActor "Human")
        (bind _asbp_rpg_enemy_base (cast `/Game/_Game/Blueprints/Character/Enemies/BP_RPG_Enemy_Base` OtherActor))
        (`/Engine/EditorBlueprintResources/StandardMacros.IsValid` _asbp_rpg_enemy_base
          (:`Is Valid`
            (`KismetArrayLibrary.Array_AddUnique` (`self.EnemyAICharacters`) _asbp_rpg_enemy_base)))))))

(event `Check if AI In Searching state`
  (bind _returnvalue (`KismetSystemLibrary.K2_SetTimerDelegate` (delegate `Check Is In Searching State`) 0.1 true))
  (set `self.CheckIsInSearchingState_TimerHandle` _returnvalue))

(event `Check Is In Searching State`
  (for _array_element (`self.EnemyAICharacters`)
    (`/Engine/EditorBlueprintResources/StandardMacros.IsValid` _array_element
      (:`Is Valid`
        (bind _inawarnedstate (message `/Game/_Game/Blueprints/Interfaces/BPI_AIController_Interface.GetAwarnedState` (`AIBlueprintHelperLibrary.GetAIController` _array_element)))
        (switch `/Game/_Game/Blueprints/Enums/E_AwarnedStates` _inawarnedstate
          (:`NewEnumerator0`
            (set `self.bAIReadyToSearch` true))
          (:`NewEnumerator1`
            (set `self.bAIReadyToSearch` false)
            (break))))))
  (if (`self.bAIReadyToSearch`)
    (`self.FindCoverForAI`)))

(event `Reset Covers`
  (`KismetSystemLibrary.K2_SetTimerDelegate` (delegate `Reset Status Of All Covers`) 0.5 true))

(event `Reset Status Of All Covers`
  (for _array_element (`self.CoverActors`)
    (if (`.bIsInvestigated_3_3E67C410452A13DD61CD20A19F9A8C64` (break `/Game/_Game/Blueprints/Structs/F_CoverStruct` (`/Game/_Game/Blueprints/Actors/AICoverSystem/BP_EnvironmentCover_Base.CoverStatus` _array_element)))
      (set `self.bCanResetCovers` true)
      (else
        (set `self.bCanResetCovers` false)
        (break))))
  (if (`self.bCanResetCovers`)
    (for _array_element_2 (`self.CoverActors`)
      (bind _output_get (set `/Game/_Game/Blueprints/Actors/AICoverSystem/BP_EnvironmentCover_Base.CoverStatus` (make `/Game/_Game/Blueprints/Structs/F_CoverStruct` false) _array_element_2))
      (bind (_bisreserved _bisinvestigated) (break `/Game/_Game/Blueprints/Structs/F_CoverStruct` _output_get))
      (`/Game/_Game/Blueprints/Actors/AICoverSystem/BP_EnvironmentCover_Base.Set Text In Widget` _array_element_2 _bisreserved _bisinvestigated))
    (set `self.bCanResetCovers` false)))

(fn `FindCoverForAI`
  (locals (TargetCover_Local :type "/Game/_Game/Blueprints/Actors/AICoverSystem/BP_EnvironmentCover_Base Object Reference") (ClosestEnemy :type "/Game/_Game/Blueprints/Character/Enemies/BP_RPG_Enemy_Base Object Reference") (ClosestDistance :type "Float (double-precision)"))
  (bind _targetcover_local (`local.TargetCover_Local`))
  (bind _targetcover_local_2 (`local.TargetCover_Local`))
  (bind (_coverstatus_bisreserved _coverstatus_bisinvestigated) (break `/Game/_Game/Blueprints/Structs/F_CoverStruct` (`/Game/_Game/Blueprints/Actors/AICoverSystem/BP_EnvironmentCover_Base.CoverStatus` _targetcover_local_2)))
  ; Check if Cover not reserved by AI and Not Investigated
  (set `local.TargetCover_Local` null)
  (for _array_element (`self.CoverActors`)
    (bind (_bisreserved _bisinvestigated) (break `/Game/_Game/Blueprints/Structs/F_CoverStruct` (`/Game/_Game/Blueprints/Actors/AICoverSystem/BP_EnvironmentCover_Base.CoverStatus` _array_element)))
    (if (and (not _bisreserved) (not _bisinvestigated))
      (set `local.TargetCover_Local` _array_element)
      (break)))
  (set `local.ClosestEnemy` null)
  (set `local.ClosestDistance` 9999999999.0)
  ; Find Closest AI Controller to Cover
  (for _array_element_2 (`self.EnemyAICharacters`)
    (`/Engine/EditorBlueprintResources/StandardMacros.IsValid` _array_element_2
      (:`Is Valid`
        (if (`|EnumEquality` (`/Game/_Game/Blueprints/Character/Enemies/BP_RPG_Enemy_Base.SearchingState` _array_element_2) "NewEnumerator0")
          (`/Engine/EditorBlueprintResources/StandardMacros.IsValid` _targetcover_local
            (:`Is Valid`
              (if (!= (`/Game/_Game/Blueprints/Character/Enemies/BP_RPG_Enemy_Base.LastInvestigatedCover` _array_element_2) (`local.TargetCover_Local`))
                (bind _returnvalue (`self.GetDistanceTo` _targetcover_local _array_element_2))
                (if (< _returnvalue (`local.ClosestDistance`))
                  (set `local.ClosestDistance` _returnvalue)
                  (set `local.ClosestEnemy` _array_element_2))))
            (:`Is Not Valid`
              (return)))))))
  (`/Engine/EditorBlueprintResources/StandardMacros.IsValid` (`local.ClosestEnemy`)
    (:`Is Valid`
      (set `/Game/_Game/Blueprints/Actors/AICoverSystem/BP_EnvironmentCover_Base.CoverStatus` (make `/Game/_Game/Blueprints/Structs/F_CoverStruct` true false (`local.ClosestEnemy`)) (`local.TargetCover_Local`))
      (`/Game/_Game/Blueprints/Actors/AICoverSystem/BP_EnvironmentCover_Base.Set Text In Widget` _targetcover_local_2 _coverstatus_bisreserved _coverstatus_bisinvestigated)
      (`/Game/_Game/Blueprints/Actors/AICoverSystem/BP_EnvironmentCover_Base.Retrigger Sphere Overlap` (`local.TargetCover_Local`))
      (set `/Game/_Game/Blueprints/Character/Enemies/BP_RPG_Enemy_Base.LastInvestigatedCover` (`local.TargetCover_Local`) (`local.ClosestEnemy`))
      (message `/Game/_Game/Blueprints/Interfaces/BPI_AIController_Interface.SetTargetCoverLocation` (`AIBlueprintHelperLibrary.GetAIController` (`local.ClosestEnemy`)) (`self.K2_GetActorLocation` (`local.TargetCover_Local`)))
      (message `/Game/_Game/Blueprints/Interfaces/BPI_AIController_Interface.SetSearchingState_Interface` (`AIBlueprintHelperLibrary.GetAIController` (`local.ClosestEnemy`)) "NewEnumerator1")
      (return))
    (:`Is Not Valid`
      (return))))

(fn `UserConstructionScript`)