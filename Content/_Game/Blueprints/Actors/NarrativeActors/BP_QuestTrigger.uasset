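; Narrative trigger volume that starts the quest set in QuestClass when the player enters its box.
; On overlap by a Player-tagged actor, it passes the class to player controller 0 through BeginQuestMessage, then disables the box's collision.
; A DoOnce keeps it single-use, resetting when a non-player overlaps or the class is invalid, with an error message for the latter.
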(event `self.BoxTrigger.OnComponentBeginOverlap`
  (params (OverlappedComponent :type "PrimitiveComponent Object Reference") (OtherActor :type "Actor Object Reference") (OtherComp :type "PrimitiveComponent Object Reference") (OtherBodyIndex :type Integer) (bFromSweep :type Boolean) (SweepResult :type "HitResult Structure (by ref)"))
  (bind _questclass (`self.QuestClass`))
  (`/Engine/EditorBlueprintResources/StandardMacros.DoOnce` false :!label _label
    (:`Completed`
      (if (`self.ActorHasTag` OtherActor "Player")
        (if (`KismetSystemLibrary.IsValidClass` _questclass)
          (message `/Game/_Game/Blueprints/Interfaces/BPI_PlayerControllerNarrative.BeginQuest` (`GameplayStatics.GetPlayerController` 0) _questclass)
          (`|ExecutionSequence`
            (:`then_0`
              (`PrimitiveComponent.SetCollisionEnabled` (`self.BoxTrigger`) "NoCollision"))
            (:`then_1`
              (`/Game/_Game/Blueprints/Libraries/BP_MicroLibrary.ErrorMessage` "Test Quest Started")))
          (else
            (`|ExecutionSequence`
              (:`then_0`
                (`/Game/_Game/Blueprints/Libraries/BP_MicroLibrary.ErrorMessage` "error! Attempt to activate a quest witch is null or pending to kill!"))
              (:`then_1`
                (goto _label :!via `Reset`)))))
        (else
          (goto _label :!via `Reset`))))))

(fn `UserConstructionScript`)