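; A narrative goal location actor that shows an exclamation-mark world marker on the HUD for a specific quest.
; On BeginPlay it builds the marker style and binds to the Narrative component's quest-started and branch-completed events.
; It registers itself with the HUD manager when a quest matching its QuestName starts.
; It removes the marker when that quest completes the branch matching its QuestStateID.
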(event `self.ReceiveBeginPlay`
  (bind _returnvalue (`NarrativeFunctionLibrary.GetNarrativeComponent`))
  ; Store World Marker Style
  (set `self.S World Marker Info` (make `/Game/ProHUDV2/Blueprints/Structs/S_WorldMarkerInfo` "/Game/ProHUDV2/DemoContent/Textures/DemoIcons/T_E_Exclamationmark_256x256.T_E_Exclamationmark_256x256" 1.0 (struct :`R` 1.0 :`G` 0.35 :`B` 0.05 :`A` 1.0) true "Go To Ledge" (struct :`FontInfo` (struct :`OutlineSettings` (struct :`OutlineColor` (struct :`A` 1.0)) :`Size` 24.0 :`MonospacedWidth` 1.0) :`Scale` 1.0 :`ColorAndOpacity` (struct)) true true (struct :`DistanceUnit` "NewEnumerator1" :`DistanceStepskm` 10 :`DistanceStepsm` 1 :`DistanceStepsmi` 10 :`DistanceStepsya` 1) (struct :`FontInfo` (struct :`OutlineSettings` (struct :`OutlineColor` (struct :`A` 1.0)) :`Size` 24.0 :`MonospacedWidth` 1.0) :`Scale` 1.0 :`ColorAndOpacity` (struct)) 0 true true))
  (add `NarrativeComponent.OnQuestStarted` _returnvalue (delegate `OnQuestStarted_Event`))
  (add `NarrativeComponent.OnQuestBranchCompleted` _returnvalue (delegate `OnQuestBranchCompleted_Event`)))

(event `OnQuestStarted_Event`
  (params (Quest :type "Quest Object Reference"))
  (if (`KismetTextLibrary.EqualEqual_TextText` (`Quest.QuestName` Quest) (`self.QuestName`))
    (`|ExecutionSequence`
      (:`then_0`
        (`/Game/ProHUDV2/Blueprints/Libraries/BPi_HUDManagerV2.AddOrUpdateWorldMarker` (`/Game/ProHUDV2/Blueprints/Libraries/BP_PHV2_Functions.GetHUDManager`) self (`self.S World Marker Info`))))))

(event `OnQuestBranchCompleted_Event`
  (params (Quest :type "Quest Object Reference") (Branch :type "QuestBranch Object Reference"))
  (if (and (`KismetTextLibrary.EqualEqual_TextText` (`Quest.QuestName` Quest) (`self.QuestName`)) (== (`NarrativeNodeBase.ID` Branch) (`self.QuestStateID`)))
    (`/Game/ProHUDV2/Blueprints/Libraries/BPi_HUDManagerV2.RemoveWorldMarker` (`/Game/ProHUDV2/Blueprints/Libraries/BP_PHV2_Functions.GetHUDManager`) self)))

(fn `UserConstructionScript`)