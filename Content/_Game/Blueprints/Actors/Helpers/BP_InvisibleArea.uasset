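; BP_InvisibleArea is a helper trigger volume that hides the player from stimulus-based detection while they stand inside it.
; When an actor tagged Player enters the Box, it casts to BP_RPG_PlayerCharacter and disables all of that character's stimuli.
; Leaving the Box re-enables them, and both transitions print a debug string.
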(event `self.Box.OnComponentBeginOverlap`
  (params (OverlappedComponent :type "PrimitiveComponent Object Reference") (OtherActor :type "Actor Object Reference") (OtherComp :type "PrimitiveComponent Object Reference") (OtherBodyIndex :type Integer) (bFromSweep :type Boolean) (SweepResult :type "HitResult Structure (by ref)"))
  (if (`self.ActorHasTag` OtherActor "Player")
    (bind _asbp_rpg_player_character (cast `/Game/_Game/Blueprints/Character/Player/BP_RPG_PlayerCharacter` OtherActor))
    (`/Engine/EditorBlueprintResources/StandardMacros.IsValid` _asbp_rpg_player_character
      (:`Is Valid`
        (`/Game/_Game/Blueprints/Character/Player/BP_RPG_PlayerCharacter.Disable All Stimulus` _asbp_rpg_player_character)
        (`KismetSystemLibrary.PrintString` "DISABLE ALL STIMULUS")))))

(event `self.Box.OnComponentEndOverlap`
  (params (OverlappedComponent :type "PrimitiveComponent Object Reference") (OtherActor :type "Actor Object Reference") (OtherComp :type "PrimitiveComponent Object Reference") (OtherBodyIndex :type Integer))
  (if (`self.ActorHasTag` OtherActor "Player")
    (bind _asbp_rpg_player_character (cast `/Game/_Game/Blueprints/Character/Player/BP_RPG_PlayerCharacter` OtherActor))
    (`/Engine/EditorBlueprintResources/StandardMacros.IsValid` _asbp_rpg_player_character
      (:`Is Valid`
        (`/Game/_Game/Blueprints/Character/Player/BP_RPG_PlayerCharacter.Enable All Stimulus` _asbp_rpg_player_character)
        (`KismetSystemLibrary.PrintString` "ENABLE ALL STIMULUS")))))

(fn `UserConstructionScript`)