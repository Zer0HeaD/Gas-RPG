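; Helper actor that manages separate melee and ranged attack token pools for a group of AI.
; Construction seeds both token components' counts, and wrapper functions forward reserve, return, melee count and closest-enemy calls to them.
; Each Tick also runs a fan of multi-sphere traces around the player pawn's forward direction, though the trace results are not used here.
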(event `self.ReceiveBeginPlay`)

(event `self.ReceiveTick`
  (params (DeltaSeconds :type "Float (single-precision)"))
  (`self.ConeTraceByChannel`))

(event `/Game/_Game/Blueprints/Interfaces/BPI_AIGroupInterface.ReturnMeleeAttackToken`
  (params (Amount :type Integer))
  (`/Game/_Game/Blueprints/Components/BP_AITokenComponent.ReturnAttackToken` (`self.MeleeTokenComponent`) Amount))

(event `/Game/_Game/Blueprints/Interfaces/BPI_AIGroupInterface.ReturnRangeAttackToken`
  (params (Amount :type Integer))
  (`/Game/_Game/Blueprints/Components/BP_AITokenComponent.ReturnAttackToken` (`self.RangeTokenComponent`) Amount))

(fn `ConeTraceByChannel`
  (locals (Location_Local :type "Vector Structure" :default (0.0 0.0 0.0)) (ForwardVector_Local :type "Vector Structure" :default (0.0 0.0 0.0)) (TraceDirections_Local :type "Array of Integer") (UpVector_Local :type "Vector Structure" :default (0.0 0.0 0.0)))
  (bind _returnvalue (`GameplayStatics.GetPlayerPawn` 0))
  (bind _returnvalue_2 (+ (`local.Location_Local`) (0.0 0.0 75.0)))
  (`/Engine/EditorBlueprintResources/StandardMacros.IsValid` _returnvalue
    (:`Is Valid`
      (set `local.Location_Local` (`self.K2_GetActorLocation` _returnvalue))
      (set `local.ForwardVector_Local` (`self.GetActorForwardVector` _returnvalue))
      (set `local.UpVector_Local` (`self.GetActorUpVector` _returnvalue))
      (for _array_element (`local.TraceDirections_Local`)
        (`KismetSystemLibrary.SphereTraceMulti` _returnvalue_2 (+ _returnvalue_2 (* (`KismetMathLibrary.RotateAngleAxis` (`local.ForwardVector_Local`) (`KismetMathLibrary.Conv_IntToDouble` _array_element) (`local.UpVector_Local`)) 2000.0)) 125.0 "TraceTypeQuery5" false (`|MakeArray` (`GameplayStatics.GetPlayerPawn` 0) :!type "Actor Object Reference")))
      (return))))

(fn `GetClosestEnemyToPlayer`
  (returns (InEnemy :type "Actor Object Reference"))
  (return (`/Game/_Game/Blueprints/Components/BP_AITokenComponent.GetClosestEnemyToPlayer` (`self.MeleeTokenComponent`))))

(fn `GetMeleeTokenCount`
  (returns (InCount :type Integer))
  (return (`/Game/_Game/Blueprints/Components/BP_AITokenComponent.GetAttackTokenCount` (`self.MeleeTokenComponent`))))

(fn `ReserveMeleeAttackToken`
  (params (Amount :type Integer))
  (returns (Success :type Boolean))
  (bind _success (`/Game/_Game/Blueprints/Components/BP_AITokenComponent.ReserveAttackToken` (`self.MeleeTokenComponent`) Amount))
  (return _success))

(fn `ReserveRangeAttackToken`
  (params (Amount :type Integer))
  (returns (Success :type Boolean))
  (bind _success (`/Game/_Game/Blueprints/Components/BP_AITokenComponent.ReserveAttackToken` (`self.RangeTokenComponent`) Amount))
  (return _success))

(fn `UserConstructionScript`
  (set `/Game/_Game/Blueprints/Components/BP_AITokenComponent.AttackTokenCount` (`self.Attack Melee Token Count`) (`self.MeleeTokenComponent`))
  (set `/Game/_Game/Blueprints/Components/BP_AITokenComponent.AttackTokenCount` (`self.Attack Range Token Count`) (`self.RangeTokenComponent`)))