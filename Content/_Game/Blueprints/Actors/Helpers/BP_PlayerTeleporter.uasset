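; BP_PlayerTeleporter is a trigger actor that resets the player's location when the player enters its box.
; An overlap by an actor tagged "Player" asks the HUD manager for a blackscreen effect and starts a delay timer.
; When the timer fires, it sends a reset-location message to player character 0 with twice the delay, leaving the actual move to the character.
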(event `self.Box.OnComponentBeginOverlap`
  (params (OverlappedComponent :type "PrimitiveComponent Object Reference") (OtherActor :type "Actor Object Reference") (OtherComp :type "PrimitiveComponent Object Reference") (OtherBodyIndex :type Integer) (bFromSweep :type Boolean) (SweepResult :type "HitResult Structure (by ref)"))
  (bind _delaybeforeresetlocationtime (`self.DelayBeforeResetLocationTime`))
  (if (`self.ActorHasTag` OtherActor "Player")
    (`/Game/ProHUDV2/Blueprints/Libraries/BPi_HUDManagerV2.CreateHUDFX_Blackscreen` (`/Game/ProHUDV2/Blueprints/Libraries/BP_PHV2_Functions.GetHUDManager`) _delaybeforeresetlocationtime)
    (bind _returnvalue (`KismetSystemLibrary.K2_SetTimerDelegate` (delegate `Reset Player's Location`) _delaybeforeresetlocationtime))
    (set `self.ResetPlayerLocation_TimerHandle` _returnvalue)))

(event `Reset Player's Location`
  (message `/Game/_Game/Blueprints/Interfaces/BPI_PlayerCharacterUtility.ResetPlayerLocation` (`GameplayStatics.GetPlayerCharacter` 0) (* (`self.DelayBeforeResetLocationTime`) 2.0)))

(fn `UserConstructionScript`)