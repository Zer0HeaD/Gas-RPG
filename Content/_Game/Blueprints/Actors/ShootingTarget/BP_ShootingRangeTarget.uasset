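; BP_ShootingRangeTarget is a shooting range target actor that tracks a down state in IsTargetDown, with its hit logic currently disconnected.
; BeginPlay starts a looping frame-delta timer that, while the target is down, re-arms a three-second timer to ResetEvent.
; ResetEvent sets IsTargetDown to true, so it never raises the target.
; The SK_Target overlap is empty; the projectile-tag check with retriggerable-delay reset is unwired.
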(event `self.ReceiveBeginPlay`
  (bind _returnvalue (`KismetSystemLibrary.K2_SetTimerDelegate` (delegate `Reset Target Event`) (`GameplayStatics.GetWorldDeltaSeconds`) true true))
  (set `self.ResetTarget_TimerHandle` _returnvalue))

(event `Reset Target Event`
  (if (`self.bIsTargetDown`)
    (`KismetSystemLibrary.K2_SetTimerDelegate` (delegate `Reset event`) 3.0 false true)))

(event `Reset event`
  (set `self.bIsTargetDown` true))

(event `self.SK_Target.OnComponentBeginOverlap`
  (params (OverlappedComponent :type "PrimitiveComponent Object Reference") (OtherActor :type "Actor Object Reference") (OtherComp :type "PrimitiveComponent Object Reference") (OtherBodyIndex :type Integer) (bFromSweep :type Boolean) (SweepResult :type "HitResult Structure (by ref)")))

(fn `UserConstructionScript`)