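; BP_Pistol is a pistol weapon actor that assembles its visual parts on top of inherited behavior.
; After running the parent construction script, it attaches Barrel, Ironsight01 and Ironsight02 to WeaponMesh at the forestock, scope and ironsight sockets, keeping relative transforms.
; Its event graph contains only disabled stub events, so it adds no runtime logic there.
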(fn `UserConstructionScript`
  (`parent.UserConstructionScript`)
  (`SceneComponent.K2_AttachToComponent` (`self.Barrel`) (`self.WeaponMesh`) "SOCKET_Forestock" "KeepRelative" "KeepRelative" "KeepRelative" true)
  (`SceneComponent.K2_AttachToComponent` (`self.Ironsight_02`) (`self.WeaponMesh`) "SOCKET_Ironsights" "KeepRelative" "KeepRelative" "KeepRelative" true)
  (`SceneComponent.K2_AttachToComponent` (`self.Ironsight_01`) (`self.WeaponMesh`) "SOCKET_Scope" "KeepRelative" "KeepRelative" "KeepRelative" true))