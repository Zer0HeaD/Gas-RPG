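; Base weapon actor that configures its mesh and the player's animation layers.
; The construction script looks up its row in DT_WeaponSettings by WeaponRowName, caches the settings and applies that row's animation Blueprint to the weapon mesh.
; On BeginPlay it links PlayerAnimInstanceClass as anim class layers on the first player's RPG_Gas_Character mesh.
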(event `self.ReceiveBeginPlay`
  (bind _asrpg_gas_character (cast `RPG_Gas_Character` (`GameplayStatics.GetPlayerPawn` 0)))
  (`/Engine/EditorBlueprintResources/StandardMacros.IsValid` _asrpg_gas_character
    (:`Is Valid`
      (`SkeletalMeshComponent.LinkAnimClassLayers` (`Character.Mesh` _asrpg_gas_character) (`self.PlayerAnimInstanceClass`)))))

(fn `UserConstructionScript`
  (bind _returnvalue (`|GetDataTableRow` "/Game/_Game/Data/ShootingData/DataTables/DT_WeaponSettings.DT_WeaponSettings" (`self.WeaponRowName`))
    (:`then`
      (bind _output_get (set `self.WeaponSettings` _returnvalue))
      (`SkeletalMeshComponent.SetAnimInstanceClass` (`self.WeaponMesh`) (`.WeaponAnimationBlueprint` (break `WeaponSettings` _output_get))))))