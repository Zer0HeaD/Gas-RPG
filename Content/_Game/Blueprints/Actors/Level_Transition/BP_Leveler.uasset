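; BP_Leveler is a level transition actor that opens its LevelToOpen level when its Tap interaction completes.
; Overlap of WidgetCollision by a "Chibi"-tagged actor sends target or clear messages, which CurrentTarget and ClearTarget forward to the info widget child actor.
; The SetWidget and SetDetail functions supply that widget's configuration, enabling only a title and subtitle from variables, with fixed colors and type.
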(event `/Game/InteractionWidgets/Blueprints/Interfaces/InteractionInterface.Current Target`
  (params (Pawn :type "Pawn Object Reference"))
  (bind _childactor (`ChildActorComponent.ChildActor` (`self.Widget`)))
  ;[1 1 1] Current target (Copy and paste this in to your own actor)
  (message `/Game/InteractionWidgets/Blueprints/Interfaces/InteractionInterface.Current Target` _childactor Pawn)
  (message `/Game/InteractionWidgets/Blueprints/Interfaces/InteractionInterface.ParentActor` _childactor self))

(event `/Game/InteractionWidgets/Blueprints/Interfaces/InteractionInterface.Clear Target`
  ;[1 1 1] Clear target (Copy and paste this in to your own actor)
  (message `/Game/InteractionWidgets/Blueprints/Interfaces/InteractionInterface.Clear Target` (`ChildActorComponent.ChildActor` (`self.Widget`))))

(event `self.Tap.OnInteractionCompleted`
  (`GameplayStatics.OpenLevelBySoftObjectPtr` (`self.LevelToOpen`)))

(event `self.WidgetCollision.OnComponentBeginOverlap`
  (params (OverlappedComponent :type "PrimitiveComponent Object Reference") (OtherActor :type "Actor Object Reference") (OtherComp :type "PrimitiveComponent Object Reference") (OtherBodyIndex :type Integer) (bFromSweep :type Boolean) (SweepResult :type "HitResult Structure (by ref)"))
  ; Show Info Widget
  (if (`self.ActorHasTag` OtherActor "Chibi")
    (message `/Game/InteractionWidgets/Blueprints/Interfaces/InteractionInterface.Current Target` self (`GameplayStatics.GetPlayerPawn` 0))))

(event `self.WidgetCollision.OnComponentEndOverlap`
  (params (OverlappedComponent :type "PrimitiveComponent Object Reference") (OtherActor :type "Actor Object Reference") (OtherComp :type "PrimitiveComponent Object Reference") (OtherBodyIndex :type Integer))
  ; Show Info Widget
  (if (`self.ActorHasTag` OtherActor "Chibi")
    (message `/Game/InteractionWidgets/Blueprints/Interfaces/InteractionInterface.Clear Target` self)))

(fn `Set Detail 1`
  (returns (`Return Value` :type Boolean) (`Detail Settings` :type "/Game/InteractionWidgets/Blueprints/Stucts/S_DetailsSettings Structure"))
  (return false))

(fn `Set Detail 2`
  (returns (`Return Value` :type Boolean) (`Detail Settings` :type "/Game/InteractionWidgets/Blueprints/Stucts/S_DetailsSettings Structure"))
  (return false))

(fn `Set Detail 3`
  (returns (`Return Value` :type Boolean) (`Detail Settings` :type "/Game/InteractionWidgets/Blueprints/Stucts/S_DetailsSettings Structure"))
  (return false))

(fn `Set Detail 4`
  (returns (`Return Value` :type Boolean) (`Detail Settings` :type "/Game/InteractionWidgets/Blueprints/Stucts/S_DetailsSettings Structure"))
  (return false))

(fn `Set Widget Amount`
  (returns (`Return Value` :type Boolean) (`Amount Value` :type Integer))
  (return false 0))

(fn `Set Widget Color`
  (returns (`Dark Color` :type "LinearColor Structure") (`Light Color` :type "LinearColor Structure"))
  (return (struct :`R` 0.040915 :`G` 0.351533 :`B` 1.0 :`A` 0.5) (struct :`R` 1.0 :`G` 0.346889 :`B` 0.019981 :`A` 0.5)))

(fn `Set Widget Key Binds`
  (returns (`Return Value` :type Boolean) (`Key Binds` :type "Array of /Game/InteractionWidgets/Blueprints/Stucts/S_KeyBinds Structure"))
  (return false))

(fn `Set Widget Level`
  (returns (`Return Value` :type Boolean) (`Level Text` :type Text))
  (return false ""))

(fn `Set Widget Sub Title`
  (returns (`Return Value` :type Boolean) (`Sub Title Text` :type Text))
  (return true (`self.Sub Title Text`)))

(fn `Set Widget Title`
  (returns (`Return Value` :type Boolean) (`Title Text` :type Text))
  (return true (`self.Title Text`)))

(fn `Set Widget Type`
  (returns (`Widget Type` :type "/Game/InteractionWidgets/Blueprints/Enums/E_WidgetTypes Enum"))
  (return "NewEnumerator0"))

(fn `UserConstructionScript`)